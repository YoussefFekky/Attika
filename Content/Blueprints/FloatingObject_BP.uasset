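; Floating physics object that the player character can be attached to, snapping to its GrabLocation socket through GrabMe.
; Each tick it applies BuoyancyFunction at four corner points, splitting the mesh mass evenly between them.
; An actor overlapping the ReleaseTriggerBox detaches the player, then the object destroys itself after a short delay.
; OnReset returns it to the transform saved at BeginPlay.
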(event OnActorBeginOverlap(ReleaseTriggerBox)
  (params (OverlappedActor :type Actor%20Object%20Reference) (OtherActor :type Actor%20Object%20Reference))
  (CallFunction|ReleaseMe)
  (Utilities|FlowControl|Delay 1.0)
  (Actor|DestroyActor))

(event EventOnReset
  (Transformation|SetActorTransform (Variables|Default|GetInitialTransform)))

(event EventBeginPlay
  (Variables|Default|SetInitialTransform (Transformation|GetActorTransform)))

(event EventTick
  (params (DeltaSeconds :type Float%20%28single-precision%29))
  (bind _mesh (Variables|Default|GetMesh))
  (bind _cornerpositions (Variables|Default|GetCornerPositions))
  (for _array_element _cornerpositions
    (CallFunction|BuoyancyFunction _mesh 418.0 (Transformation|GetWorldLocation _array_element) (/ (Physics|GetMass _mesh) (Math|Conversions|ToFloat(Integer) (Utilities|Array|Length _cornerpositions))) "ObjectTypeQuery7")))

(fn ConstructionScript
  (Variables|Default|SetCornerPositions (Utilities|Array|MakeArray (Variables|Default|GetCornerPosition1) (Variables|Default|GetCornerPosition2) (Variables|Default|GetCornerPosition3) (Variables|Default|GetCornerPosition4)))
  (Variables|Default|SetObjectTypes (Utilities|Array|MakeArray (Utilities|Enum|LiteralenumEObjectTypeQuery "ObjectTypeQuery4"))))

(fn GrabMe
  (bind _asthird_person_character (Utilities|Casting|CastToThirdPersonCharacter (Game|GetPlayerCharacter 0)))
  (bind _output_get (Variables|Default|SetGrabbedCharacter _asthird_person_character))
  (Transformation|AttachActorToActor _output_get self "GrabLocation" "SnapToTarget" "SnapToTarget" "KeepWorld" true)
  (return))

(fn ReleaseMe
  (bind _asthird_person_character (Utilities|Casting|CastToThirdPersonCharacter (Game|GetPlayerCharacter 0)))
  (Transformation|DetachFromActor _asthird_person_character "KeepWorld" "KeepRelative" "KeepWorld"))