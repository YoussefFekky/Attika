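; Pushable box actor with a lock that the third-person character can open with a key.
; Four side triggers flag which side is overlapped and set the character's push direction along the matching axis; no movement happens here.
; Tick polls the lock trigger for F pressed and key held, then sets the character's lock-open flag.
; A boolean gate limits the lock and chain-drop sounds to one play.
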(event OnComponentBeginOverlap(OpenLockCollisionBox)
  (params (OverlappedComponent :type Primitive%20Component%20Object%20Reference) (OtherActor :type Actor%20Object%20Reference) (OtherComp :type Primitive%20Component%20Object%20Reference) (OtherBodyIndex :type Integer) (bFromSweep :type Boolean) (SweepResult :type Hit%20Result%20Structure%20%28by%20ref%29))
  (bind _asthird_person_character (Utilities|Casting|CastToThirdPersonCharacter OtherActor))
  (Variables|Default|SetIsOverlappingLockPos true))

(event OnComponentEndOverlap(OpenLockCollisionBox)
  (params (OverlappedComponent :type Primitive%20Component%20Object%20Reference) (OtherActor :type Actor%20Object%20Reference) (OtherComp :type Primitive%20Component%20Object%20Reference) (OtherBodyIndex :type Integer))
  (Utilities|Casting|CastToThirdPersonCharacter OtherActor)
  (Variables|Default|SetIsOverlappingLockPos false))

(event OnComponentEndOverlap(Side4)
  (params (OverlappedComponent :type Primitive%20Component%20Object%20Reference) (OtherActor :type Actor%20Object%20Reference) (OtherComp :type Primitive%20Component%20Object%20Reference) (OtherBodyIndex :type Integer))
  (Utilities|Casting|CastToThirdPersonCharacter OtherActor)
  (Variables|Default|SetSide_4 false))

(event OnComponentBeginOverlap(Side1)
  (params (OverlappedComponent :type Primitive%20Component%20Object%20Reference) (OtherActor :type Actor%20Object%20Reference) (OtherComp :type Primitive%20Component%20Object%20Reference) (OtherBodyIndex :type Integer) (bFromSweep :type Boolean) (SweepResult :type Hit%20Result%20Structure%20%28by%20ref%29))
  (bind _asthird_person_character (Utilities|Casting|CastToThirdPersonCharacter OtherActor))
  (Variables|Default|SetSide_1 true)
  (Variables|/Game/ThirdPersonBP/Blueprints/ThirdPersonCharacter.ThirdPersonCharacter_C|SetSetPushDirection _asthird_person_character "-1.000000, 0, 0"))

(event OnComponentBeginOverlap(Side2)
  (params (OverlappedComponent :type Primitive%20Component%20Object%20Reference) (OtherActor :type Actor%20Object%20Reference) (OtherComp :type Primitive%20Component%20Object%20Reference) (OtherBodyIndex :type Integer) (bFromSweep :type Boolean) (SweepResult :type Hit%20Result%20Structure%20%28by%20ref%29))
  (bind _asthird_person_character (Utilities|Casting|CastToThirdPersonCharacter OtherActor))
  (Variables|Default|SetSide_2 true)
  (Variables|/Game/ThirdPersonBP/Blueprints/ThirdPersonCharacter.ThirdPersonCharacter_C|SetSetPushDirection _asthird_person_character "0.000000,1.000000, 0"))

(event OnComponentEndOverlap(Side2)
  (params (OverlappedComponent :type Primitive%20Component%20Object%20Reference) (OtherActor :type Actor%20Object%20Reference) (OtherComp :type Primitive%20Component%20Object%20Reference) (OtherBodyIndex :type Integer))
  (Utilities|Casting|CastToThirdPersonCharacter OtherActor)
  (Variables|Default|SetSide_2 false))

(event OnComponentEndOverlap(Side1)
  (params (OverlappedComponent :type Primitive%20Component%20Object%20Reference) (OtherActor :type Actor%20Object%20Reference) (OtherComp :type Primitive%20Component%20Object%20Reference) (OtherBodyIndex :type Integer))
  (Utilities|Casting|CastToThirdPersonCharacter OtherActor)
  (Variables|Default|SetSide_1 false))

(event OnComponentBeginOverlap(Side3)
  (params (OverlappedComponent :type Primitive%20Component%20Object%20Reference) (OtherActor :type Actor%20Object%20Reference) (OtherComp :type Primitive%20Component%20Object%20Reference) (OtherBodyIndex :type Integer) (bFromSweep :type Boolean) (SweepResult :type Hit%20Result%20Structure%20%28by%20ref%29))
  (bind _asthird_person_character (Utilities|Casting|CastToThirdPersonCharacter OtherActor))
  (Variables|Default|SetSide_3 true)
  (Variables|/Game/ThirdPersonBP/Blueprints/ThirdPersonCharacter.ThirdPersonCharacter_C|SetSetPushDirection _asthird_person_character "1.000000,0.000000, 0"))

(event OnComponentEndOverlap(Side3)
  (params (OverlappedComponent :type Primitive%20Component%20Object%20Reference) (OtherActor :type Actor%20Object%20Reference) (OtherComp :type Primitive%20Component%20Object%20Reference) (OtherBodyIndex :type Integer))
  (Utilities|Casting|CastToThirdPersonCharacter OtherActor)
  (Variables|Default|SetSide_3 false))

(event OnComponentBeginOverlap(Side4)
  (params (OverlappedComponent :type Primitive%20Component%20Object%20Reference) (OtherActor :type Actor%20Object%20Reference) (OtherComp :type Primitive%20Component%20Object%20Reference) (OtherBodyIndex :type Integer) (bFromSweep :type Boolean) (SweepResult :type Hit%20Result%20Structure%20%28by%20ref%29))
  (bind _asthird_person_character (Utilities|Casting|CastToThirdPersonCharacter OtherActor))
  (Variables|Default|SetSide_4 true)
  (Variables|/Game/ThirdPersonBP/Blueprints/ThirdPersonCharacter.ThirdPersonCharacter_C|SetSetPushDirection _asthird_person_character "0.000000,-1.000000, 0"))

(event EventTick
  (params (DeltaSeconds :type Float%20%28single-precision%29))
  (if (Variables|Default|GetIsOverlappingLockPos)
    (if (and (Variables|/Game/ThirdPersonBP/Blueprints/ThirdPersonCharacter.ThirdPersonCharacter_C|GetFispressed (stale OnComponentBeginOverlap(OpenLockCollisionBox) _asthird_person_character)) (Variables|/Game/ThirdPersonBP/Blueprints/ThirdPersonCharacter.ThirdPersonCharacter_C|GetHasKey (stale OnComponentBeginOverlap(OpenLockCollisionBox) _asthird_person_character)))
      (Variables|/Game/ThirdPersonBP/Blueprints/ThirdPersonCharacter.ThirdPersonCharacter_C|SetIsLockOpen (stale OnComponentBeginOverlap(OpenLockCollisionBox) _asthird_person_character) true)
      (if (Variables|Default|Getplaysound)
        (Variables|Default|Setplaysound false)
        (Audio|Components|Audio|Play (Variables|Default|GetModifiedLock_opening_lite04_Cue) 0.0)
        (Audio|Components|Audio|Play (Variables|Default|GetChainDrop) 0.0)))))

(fn ConstructionScript)