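; Hidden door Blueprint that sinks into the ground with a sliding sound and waterfall effect when OpenDoor is called.
; The construction script caches the door's position and derives an open position one full bounds height below it.
; Separate timelines lerp the door down and, after a delay, back up, then deactivate the waterfall.
; A DoOnce with no reset limits the automatic close to a single time.
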(event Custom|OpenDoor
  (bind _initialposition (Variables|Default|GetInitialPosition))
  (Audio|PlaySoundatLocation "/Game/Sounds/PureSounds/LargeWoodenObject_Sliding_01_04.LargeWoodenObject_Sliding_01_04" _initialposition "0, 0, 0" 1.0 1.0 0.0 0 0 0)
  (Components|Activation|SetActive (Variables|Default|GetWaterfall) true false)
  (bind _lerp (Timeline|DoorLowerTimeline Play)
    (:Update
      (Transformation|SetWorldLocation (Variables|Default|GetDoor) (Math|Vector|Lerp(Vector) _initialposition (Variables|Default|GetOpenPosition) _lerp) false false))
    (:Finished
      (Utilities|FlowControl|DoOnce false
        (:Completed
          (Utilities|FlowControl|Delay 3.0)
          (Audio|PlaySoundatLocation "/Game/Sounds/PureSounds/LargeWoodenObject_Sliding_01_04.LargeWoodenObject_Sliding_01_04" _initialposition "0, 0, 0" 1.0 1.0 0.0 0 0 0)
          (bind _lerp_2 (Timeline|CloseDoor_TL Play)
            (:Update
              (Transformation|SetWorldLocation (Variables|Default|GetDoor) (Math|Vector|Lerp(Vector) (Variables|Default|GetOpenPosition) (Variables|Default|GetInitialPosition) _lerp_2) false false))
            (:Finished
              (Components|Activation|SetActive (Variables|Default|GetWaterfall) false false))))))))

(fn ConstructionScript
  (bind _door (Variables|Default|GetDoor))
  (bind _returnvalue (Transformation|GetWorldLocation _door))
  (bind (_x _y _z) (Math|Vector|BreakVector _returnvalue))
  (Variables|Default|SetInitialPosition _returnvalue)
  (Variables|Default|SetOpenPosition (Math|Vector|MakeVector _x _y (- _z (* (.z (.BoxExtent (Collision|GetComponentBounds (Variables|Default|GetDoor)))) 2.0)))))