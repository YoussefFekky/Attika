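; Interactable picture that acts as a hidden switch, opening a secret door when the player uses it.
; The trigger volume shows or hides an interact prompt as the player enters or leaves.
; Tick polls the overlap and the player's IsInteracting flag, then once only hides the prompt and plays a sliding sound.
; A timeline rotates the picture incrementally on each update, then calls OpenDoor on HiddenDoor when finished.
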(event OnComponentBeginOverlap(PictureTrigger)
  (params (OverlappedComponent :type Primitive%20Component%20Object%20Reference) (OtherActor :type Actor%20Object%20Reference) (OtherComp :type Primitive%20Component%20Object%20Reference) (OtherBodyIndex :type Integer) (bFromSweep :type Boolean) (SweepResult :type Hit%20Result%20Structure%20%28by%20ref%29))
  (Utilities|Casting|CastToThirdPersonCharacter OtherActor)
  (Rendering|SetVisibility (Variables|Default|GetInteractButton) true false))

(event OnComponentEndOverlap(PictureTrigger)
  (params (OverlappedComponent :type Primitive%20Component%20Object%20Reference) (OtherActor :type Actor%20Object%20Reference) (OtherComp :type Primitive%20Component%20Object%20Reference) (OtherBodyIndex :type Integer))
  (Utilities|Casting|CastToThirdPersonCharacter OtherActor)
  (Rendering|SetVisibility (Variables|Default|GetInteractButton) false false))

(event EventBeginPlay
  (bind _asthird_person_character (Utilities|Casting|CastToThirdPersonCharacter (Game|GetPlayerCharacter 0)))
  (Variables|Default|SetPlayerCharacter _asthird_person_character))

(event EventTick
  (params (DeltaSeconds :type Float%20%28single-precision%29))
  (bind _playercharacter (Variables|Default|GetPlayerCharacter))
  (if (Collision|IsOverlappingActor (Variables|Default|GetPictureTrigger) _playercharacter :!class /Script/Engine.PrimitiveComponent)
    (if (Variables|/Game/ThirdPersonBP/Blueprints/ThirdPersonCharacter.ThirdPersonCharacter_C|GetIsInteracting _playercharacter)
      (Utilities|FlowControl|DoOnce false
        (:Completed
          (Development|SetHiddeninGame (Variables|Default|GetInteractButton) true false)
          (Audio|PlaySoundatLocation "/Game/Sounds/PureSounds/SlidingPicture.SlidingPicture" (Transformation|GetWorldLocation (Variables|Default|GetPicture)) "0, 0, 0" 2.0 1.0 0.0 0 0 0)
          (Timeline|PictureRotate_TL Play
            (:Update
              (Transformation|AddRelativeRotation (Variables|Default|GetPicture) "0, 0,1.000000" false false))
            (:Finished
              (Default|OpenDoor (Variables|Default|GetHiddenDoor)))))))))

(fn ConstructionScript)