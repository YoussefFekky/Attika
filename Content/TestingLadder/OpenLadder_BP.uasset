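; Folding two-part ladder actor that swings open through timelines and lets the ThirdPersonCharacter climb up or down it.
; Tick starts the character's climb trace at the bottom, while top overlap boxes trigger climbing off or, once opened, mounting from above.
; Chained timelines nudge the character into place while setting movement modes and AnimBP flags.
; PlayerIsTop toggles which trigger boxes generate overlaps.
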(event OnComponentBeginOverlap(TopEnter)
  (params (OverlappedComponent :type Primitive%20Component%20Object%20Reference) (OtherActor :type Actor%20Object%20Reference) (OtherComp :type Primitive%20Component%20Object%20Reference) (OtherBodyIndex :type Integer) (bFromSweep :type Boolean) (SweepResult :type Hit%20Result%20Structure%20%28by%20ref%29))
  (bind _char (Variables|Default|GetChar))
  (bind _char_2 (Variables|Default|GetChar))
  (bind _char_3 (Variables|Default|GetChar))
  (if (Variables|Default|GetLadder_is_Opened)
    (bind _asthird_person_character (Utilities|Casting|CastToThirdPersonCharacter OtherActor))
    (Variables|/Game/ThirdPersonBP/Blueprints/ThirdPersonCharacter.ThirdPersonCharacter_C|SetLadderBP _asthird_person_character self)
    (Pawn|Components|CharacterMovement|SetMovementMode (Variables|/Script/Engine.Character|GetCharacterMovement (Variables|Default|GetChar)) "MOVE_None" 0)
    (Timeline|Timeline_5_0 PlayFromStart
      (:Update
        (bind (_location _rotation) (CallFunction|AdjustPLayerLocation&Rotation _char))
        (Transformation|SetActorLocationAndRotation _char _location _rotation))
      (:Finished
        (Pawn|Components|CharacterMovement|SetMovementMode (Variables|/Script/Engine.Character|GetCharacterMovement (Variables|Default|GetChar)) "MOVE_Flying" 0)
        (Variables|/Game/ThirdPersonBP/Amy/Character_Anim_BP.Character_Anim_BP_C|SetDescendingTopLadder (Variables|/Game/ThirdPersonBP/Blueprints/ThirdPersonCharacter.ThirdPersonCharacter_C|GetANIM_BP _asthird_person_character) true)
        (Timeline|Timeline_6 PlayFromStart
          (:Finished
            (Timeline|Timeline_3_0 PlayFromStart
              (:Update
                (Transformation|SetActorLocation _char_3 (+ (Transformation|GetActorLocation _char_3) (* (Math|Vector|NegateVector (Transformation|GetActorForwardVector)) 0.6)) false false))
              (:Finished
                (Timeline|Timeline_4_0 PlayFromStart
                  (:Update
                    (Transformation|SetActorLocation _char_2 (+ (Transformation|GetActorLocation (Variables|Default|GetChar)) "0, 0,-2.500000") false false))
                  (:Finished
                    (Variables|/Game/ThirdPersonBP/Blueprints/ThirdPersonCharacter.ThirdPersonCharacter_C|SetClimbMode _char_2 true)
                    (Variables|/Game/ThirdPersonBP/Amy/Character_Anim_BP.Character_Anim_BP_C|SetCanClimb (Variables|/Game/ThirdPersonBP/Blueprints/ThirdPersonCharacter.ThirdPersonCharacter_C|GetANIM_BP _asthird_person_character) true)
                    (Variables|/Game/ThirdPersonBP/Amy/Character_Anim_BP.Character_Anim_BP_C|SetDescendingTopLadder (Variables|/Game/ThirdPersonBP/Blueprints/ThirdPersonCharacter.ThirdPersonCharacter_C|GetANIM_BP _asthird_person_character) false)
                    (Variables|Default|SetPlayer_Is_Top false)
                    (CallFunction|ToggleBoxes)))))))))))

(event OnComponentBeginOverlap(Top_Leave)
  (params (OverlappedComponent :type Primitive%20Component%20Object%20Reference) (OtherActor :type Actor%20Object%20Reference) (OtherComp :type Primitive%20Component%20Object%20Reference) (OtherBodyIndex :type Integer) (bFromSweep :type Boolean) (SweepResult :type Hit%20Result%20Structure%20%28by%20ref%29))
  (bind _char (Variables|Default|GetChar))
  (bind _asthird_person_character (Utilities|Casting|CastToThirdPersonCharacter OtherActor))
  (if (Variables|/Game/ThirdPersonBP/Blueprints/ThirdPersonCharacter.ThirdPersonCharacter_C|GetClimbMode _asthird_person_character)
    (Variables|/Game/ThirdPersonBP/Amy/Character_Anim_BP.Character_Anim_BP_C|SetClimbTopLadder (Variables|/Game/ThirdPersonBP/Blueprints/ThirdPersonCharacter.ThirdPersonCharacter_C|GetANIM_BP _asthird_person_character) true)
    (Timeline|Timeline_1_0 PlayFromStart
      (:Update
        (Transformation|SetActorLocation _char (+ (Transformation|GetActorLocation _char) "0, 0,1.280000") false false))
      (:Finished
        (Timeline|Timeline_2_0 PlayFromStart
          (:Update
            (Transformation|SetActorLocation _char (+ (Transformation|GetActorLocation _char) (* (Transformation|GetActorForwardVector) 1.4)) false false))
          (:Finished
            (Variables|/Game/ThirdPersonBP/Amy/Character_Anim_BP.Character_Anim_BP_C|SetClimbTopLadder (Variables|/Game/ThirdPersonBP/Blueprints/ThirdPersonCharacter.ThirdPersonCharacter_C|GetANIM_BP _asthird_person_character) false)
            (Variables|/Game/ThirdPersonBP/Amy/Character_Anim_BP.Character_Anim_BP_C|SetCanClimb (Variables|/Game/ThirdPersonBP/Blueprints/ThirdPersonCharacter.ThirdPersonCharacter_C|GetANIM_BP _asthird_person_character) false)
            (Pawn|Components|CharacterMovement|SetMovementMode (Variables|/Script/Engine.Character|GetCharacterMovement (Variables|Default|GetChar)) "MOVE_Walking" 0)
            (Variables|/Game/ThirdPersonBP/Blueprints/ThirdPersonCharacter.ThirdPersonCharacter_C|SetClimbMode (Variables|Default|GetChar) false)
            (Variables|Default|SetPlayer_Is_Top true)
            (CallFunction|ToggleBoxes)))))))

(event Custom|Open_Ladder
  (bind _openladder (Timeline|LadderOpen Play)
    (:Update
      (Transformation|SetWorldRotation (Variables|Default|GetLadder) (Math|Rotator|CombineRotators (Math|Rotator|MakeRotator 0.0 _openladder 0.0) (Variables|Default|Get1st_part_Init_Rotation)) false false)
      (bind _openladder_2 (Timeline|2nd_Part Play)
        (:Update
          (Transformation|SetWorldRotation (Variables|Default|Get2ndPart_Ladder) (Math|Rotator|CombineRotators (Math|Rotator|MakeRotator 0.0 _openladder_2 0.0) (Variables|Default|Get1st_part_Init_Rotation)) false false)
          (Variables|Default|SetLadder_is_Opened true))))))

(event EventBeginPlay
  (Variables|Default|Set1st_part_Init_Rotation (Transformation|GetActorRotation))
  (Collision|SetCollisionObjectType (Variables|Default|GetLadder_1st) "ECC_GameTraceChannel3")
  (Collision|SetCollisionObjectType (Variables|Default|GetLadder_2nd) "ECC_GameTraceChannel3")
  (CallFunction|ToggleBoxes)
  (bind _asthird_person_character (Utilities|Casting|CastToThirdPersonCharacter (Game|GetPlayerCharacter 0)))
  (bind _output_get (Variables|Default|SetChar _asthird_person_character))
  (Variables|Default|SetAnimBP (Variables|/Game/ThirdPersonBP/Blueprints/ThirdPersonCharacter.ThirdPersonCharacter_C|GetANIM_BP _output_get)))

(event EventTick
  (params (DeltaSeconds :type Float%20%28single-precision%29))
  (bind _returnvalue (Game|GetPlayerCharacter 0))
  (bind _asthird_person_character (Utilities|Casting|CastToThirdPersonCharacter _returnvalue))
  (if (and (Collision|IsOverlappingActor (Variables|Default|GetBottom_Enter) _returnvalue :!class /Script/Engine.PrimitiveComponent) (Variables|/Game/ThirdPersonBP/Blueprints/ThirdPersonCharacter.ThirdPersonCharacter_C|GetTryClimb _asthird_person_character))
    (Default|ClimbTrace _asthird_person_character)
    (if (Variables|/Game/ThirdPersonBP/Blueprints/ThirdPersonCharacter.ThirdPersonCharacter_C|GetClimbMode (Variables|Default|GetChar))
      _)))

(fn ConstructionScript)

(fn ToggleBoxes
  (bind _player_is_top (Variables|Default|GetPlayer_Is_Top))
  (bind _returnvalue (not _player_is_top))
  (Variables|/Script/Engine.PrimitiveComponent|SetbGenerateOverlapEvents (Variables|Default|GetBottom_Enter) _returnvalue)
  (Variables|/Script/Engine.PrimitiveComponent|SetbGenerateOverlapEvents (Variables|Default|GetTop_Leave) _returnvalue)
  (Variables|/Script/Engine.PrimitiveComponent|SetbGenerateOverlapEvents (Variables|Default|GetTopEnter) _player_is_top))

(fn AdjustPLayerLocation&Rotation
  (params (Character :type Third%20Person%20Character%20Object%20Reference))
  (bind _returnvalue (Transformation|GetActorLocation Character))
  (bind _ladder (Variables|Default|GetLadder))
  (bind _returnvalue_2 (Transformation|GetWorldLocation _ladder))
  (return (Math|Interpolation|VInterptoConstant _returnvalue (+ (* (Math|Vector|Normalize (- (+ (Math|Vector|MakeVector 0.0 0.0 (Variables|/Script/Engine.CapsuleComponent|GetCapsuleHalfHeight (Variables|/Script/Engine.Character|GetCapsuleComponent Character))) _returnvalue_2) _returnvalue)) 1.1e+02) _returnvalue_2) (Utilities|Time|GetWorldDeltaSeconds) 5e+01) (Class|KismetMathLibrary|RInterptoConstant (Transformation|GetActorRotation Character) (Transformation|GetWorldRotation (Variables|Default|GetScene)) (Utilities|Time|GetWorldDeltaSeconds) 1e+02)))