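; Attic ladder actor that swings open in two sections when its Open_Ladder event is called.
; The LadderOpen timeline pitches the Ladder component and, on each update, calls Play on the 2nd_Part timeline, which pitches 2ndPartLadder.
; Both pitches are combined with the actor rotation cached at BeginPlay and applied as world rotations.
; The graph contains no closing logic.
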(event Custom|Open_Ladder
  (bind _openladder (Timeline|LadderOpen Play)
    (:Update
      (Transformation|SetWorldRotation (Variables|Default|GetLadder) (Math|Rotator|CombineRotators (Math|Rotator|MakeRotator 0.0 _openladder 0.0) (Variables|Default|Get1st_part_Init_Rotation)) false false)
      (bind _openladder_2 (Timeline|2nd_Part Play)
        (:Update
          (Transformation|SetWorldRotation (Variables|Default|Get2ndPart_Ladder) (Math|Rotator|CombineRotators (Math|Rotator|MakeRotator 0.0 _openladder_2 0.0) (Variables|Default|Get1st_part_Init_Rotation)) false false))))))

(event EventBeginPlay
  (Variables|Default|Set1st_part_Init_Rotation (Transformation|GetActorRotation)))

(event Collision|EventActorBeginOverlap
  (params (OtherActor :type Actor%20Object%20Reference)))

(event EventTick
  (params (DeltaSeconds :type Float%20%28single-precision%29)))

(fn ConstructionScript)