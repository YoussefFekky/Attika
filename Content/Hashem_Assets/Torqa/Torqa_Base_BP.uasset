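; Torqa base actor Blueprint that continuously flickers its spotlight on and off.
; BeginPlay caches the SpotLight's starting intensity as OriginalIntensity.
; Tick runs through a short Delay as a repeating timer, then calls ToggleIntensity, which flips LightOn and switches the intensity between zero and the cached value.
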(event EventBeginPlay
  (Variables|Default|SetOriginal_Intensity (Variables|/Script/Engine.LightComponentBase|GetIntensity (Variables|Default|GetSpotLight))))

(event Collision|EventActorBeginOverlap
  (params (OtherActor :type Actor%20Object%20Reference)))

(event EventTick
  (params (DeltaSeconds :type Float%20%28single-precision%29))
  (Utilities|FlowControl|Delay 0.1)
  (CallFunction|ToggleIntensity))

(fn ConstructionScript)

(fn ToggleIntensity
  (if (Variables|Default|GetLightOn)
    (Rendering|Components|Light|SetIntensity (Variables|Default|GetSpotLight) 0.0)
    (else
      (Rendering|Components|Light|SetIntensity (Variables|Default|GetSpotLight) (Variables|Default|GetOriginal_Intensity))))
  (Variables|Default|SetLightOn (not (Variables|Default|GetLightOn))))