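; LeftWall_BP is a level actor that turns the third-person character's camera while the character is inside its RotateCamera overlap component.
; On begin overlap it stores the character's CameraBoom and plays a timeline that lerps the boom's relative yaw by ten degrees at fixed pitch.
; On end overlap the same timeline reverses, easing the camera back.
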(event OnComponentBeginOverlap(RotateCamera)
  (params (OverlappedComponent :type Primitive%20Component%20Object%20Reference) (OtherActor :type Actor%20Object%20Reference) (OtherComp :type Primitive%20Component%20Object%20Reference) (OtherBodyIndex :type Integer) (bFromSweep :type Boolean) (SweepResult :type Hit%20Result%20Structure%20%28by%20ref%29))
  (bind _asthird_person_character (Utilities|Casting|CastToThirdPersonCharacter OtherActor))
  (Variables|Default|SetCharacterCameraBoom (Variables|/Game/ThirdPersonBP/Blueprints/ThirdPersonCharacter.ThirdPersonCharacter_C|GetCameraBoom _asthird_person_character))
  (bind _alpha (Timeline|Timeline_0 Play)
    (:Update
      (Transformation|SetRelativeRotation (Variables|Default|GetCharacterCameraBoom) (Math|Rotator|Lerp(Rotator) "-15.000000,-80.000000,0.000103" "-15.000000,-90.000000,0.000103" _alpha true) false false))))

(event OnComponentEndOverlap(RotateCamera)
  (params (OverlappedComponent :type Primitive%20Component%20Object%20Reference) (OtherActor :type Actor%20Object%20Reference) (OtherComp :type Primitive%20Component%20Object%20Reference) (OtherBodyIndex :type Integer))
  (bind _asthird_person_character (Utilities|Casting|CastToThirdPersonCharacter OtherActor))
  (Variables|Default|SetCharacterCameraBoom (Variables|/Game/ThirdPersonBP/Blueprints/ThirdPersonCharacter.ThirdPersonCharacter_C|GetCameraBoom _asthird_person_character))
  (bind _alpha (Timeline|Timeline_0 Reverse)
    (:Update
      (Transformation|SetRelativeRotation (Variables|Default|GetCharacterCameraBoom) (Math|Rotator|Lerp(Rotator) "-15.000000,-80.000000,0.000103" "-15.000000,-90.000000,0.000103" _alpha true) false false))))

(fn ConstructionScript)